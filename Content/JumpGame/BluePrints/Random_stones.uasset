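; Random_stones is a stone actor for the jump game that spawns another copy of itself when the player character hits it.
; The Stone component's hit event picks a random world position, with each axis ranging from the stone's own coordinate times DistenceMultiply to a fixed cap, lower for height.
; The spawn adjusts for collisions or is skipped if blocked, and the original stone stays with no guard against repeated hits.
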(event `self.Stone.OnComponentHit`
  (params (HitComponent :type "PrimitiveComponent Object Reference") (OtherActor :type "Actor Object Reference") (OtherComp :type "PrimitiveComponent Object Reference") (NormalImpulse :type "Vector Structure") (Hit :type "HitResult Structure (by ref)"))
  (bind (_returnvalue_x _returnvalue_y _returnvalue_z) (`KismetMathLibrary.BreakVector` (`self.K2_GetActorLocation`)))
  (bind _distence_multiply_ (`self.distence multiply `))
  (cast `/Game/ThirdPerson/Blueprints/BP_ThirdPersonCharacter` OtherActor)
  (`|SpawnActorFromClass` "Random_stones_C" (`KismetMathLibrary.MakeTransform` (`KismetMathLibrary.MakeVector` (`KismetMathLibrary.Conv_Int64ToDouble` (`KismetMathLibrary.RandomInteger64InRange` (`KismetMathLibrary.Conv_DoubleToInt64` (* _returnvalue_x _distence_multiply_)) 1000)) (`KismetMathLibrary.Conv_Int64ToDouble` (`KismetMathLibrary.RandomInteger64InRange` (`KismetMathLibrary.Conv_DoubleToInt64` (* _returnvalue_y _distence_multiply_)) 1000)) (`KismetMathLibrary.Conv_Int64ToDouble` (`KismetMathLibrary.RandomInteger64InRange` (`KismetMathLibrary.Conv_DoubleToInt64` (* _returnvalue_z _distence_multiply_)) 250)))) "AdjustIfPossibleButDontSpawnIfColliding" "MultiplyWithRoot" null null))

(fn `UserConstructionScript`)