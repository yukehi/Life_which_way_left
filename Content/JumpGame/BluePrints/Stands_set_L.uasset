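; Stands_set_L is a jump-game stand set that procedurally spawns more platforms when the player character hits its Stand5 or Stand3 component.
; Each hit spawns a Standts and a Stnads_uppers actor at random world locations, adjusted or skipped on collision.
; Standts ranges derive from the character's location for Stand5 and the set's for Stand3, while Stnads_uppers uses fixed bounds.
; Nothing limits repeated hits from spawning again.
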(event `self.ReceiveBeginPlay`)

(event `self.Stand5.OnComponentHit`
  (params (HitComponent :type "PrimitiveComponent Object Reference") (OtherActor :type "Actor Object Reference") (OtherComp :type "PrimitiveComponent Object Reference") (NormalImpulse :type "Vector Structure") (Hit :type "HitResult Structure (by ref)"))
  (bind _returnvalue (`KismetMathLibrary.Conv_IntToInt64` (`self.Min`)))
  (bind _returnvalue_2 (`KismetMathLibrary.Conv_IntToInt64` (`self.Max_X`)))
  ;[1 1 1] instance Spwan stand 1
  (bind _asbp_third_person_character (cast `/Game/ThirdPerson/Blueprints/BP_ThirdPersonCharacter` OtherActor))
  (`|ExecutionSequence`
    (:`then_0`
      (bind (_returnvalue_x _returnvalue_y _returnvalue_z) (`KismetMathLibrary.BreakVector` (`self.K2_GetActorLocation` _asbp_third_person_character)))
      (`|SpawnActorFromClass` "/Game/JumpGame/BluePrints/Standts.Standts_C" (`KismetMathLibrary.MakeTransform` (`KismetMathLibrary.MakeVector` (`KismetMathLibrary.Conv_Int64ToDouble` (`KismetMathLibrary.RandomInteger64InRange` (/ (`KismetMathLibrary.Conv_DoubleToInt64` _returnvalue_x) _returnvalue_2) _returnvalue_2)) (`KismetMathLibrary.Conv_Int64ToDouble` (`KismetMathLibrary.RandomInteger64InRange` (/ (`KismetMathLibrary.Conv_DoubleToInt64` _returnvalue_y) _returnvalue_2) _returnvalue_2)) (`KismetMathLibrary.Conv_Int64ToDouble` (`KismetMathLibrary.RandomInteger64InRange` (`KismetMathLibrary.Conv_DoubleToInt64` _returnvalue_z) 250)))) "AdjustIfPossibleButDontSpawnIfColliding" "OverrideRootScale" null null))
    (:`then_1`
      (`|SpawnActorFromClass` "/Game/JumpGame/BluePrints/stnads_uppers.stnads_uppers_C" (`KismetMathLibrary.MakeTransform` (`KismetMathLibrary.MakeVector` (`KismetMathLibrary.Conv_Int64ToDouble` (`KismetMathLibrary.RandomInteger64InRange` _returnvalue _returnvalue_2)) (`KismetMathLibrary.Conv_Int64ToDouble` (`KismetMathLibrary.RandomInteger64InRange` _returnvalue _returnvalue_2)) (`KismetMathLibrary.Conv_Int64ToDouble` (`KismetMathLibrary.RandomInteger64InRange` -250 200)))) "AdjustIfPossibleButDontSpawnIfColliding" "OverrideRootScale" null null))))

(event `self.Stand3.OnComponentHit`
  (params (HitComponent :type "PrimitiveComponent Object Reference") (OtherActor :type "Actor Object Reference") (OtherComp :type "PrimitiveComponent Object Reference") (NormalImpulse :type "Vector Structure") (Hit :type "HitResult Structure (by ref)"))
  (bind (_returnvalue_x _returnvalue_y _returnvalue_z) (`KismetMathLibrary.BreakVector` (`self.K2_GetActorLocation`)))
  (bind _returnvalue (`KismetMathLibrary.Conv_IntToInt64` (`self.Min`)))
  (bind _returnvalue_2 (`KismetMathLibrary.Conv_IntToInt64` (`self.Max_X`)))
  ;[1 1 1] Spwen stand 2
  (bind _asbp_third_person_character (cast `/Game/ThirdPerson/Blueprints/BP_ThirdPersonCharacter` OtherActor))
  (`|ExecutionSequence`
    (:`then_0`
      (`|SpawnActorFromClass` "/Game/JumpGame/BluePrints/Standts.Standts_C" (`KismetMathLibrary.MakeTransform` (`KismetMathLibrary.MakeVector` (`KismetMathLibrary.Conv_Int64ToDouble` (`KismetMathLibrary.RandomInteger64InRange` _returnvalue (`KismetMathLibrary.Conv_DoubleToInt64` _returnvalue_x))) (`KismetMathLibrary.Conv_Int64ToDouble` (`KismetMathLibrary.RandomInteger64InRange` _returnvalue (`KismetMathLibrary.Conv_DoubleToInt64` _returnvalue_y))) (`KismetMathLibrary.Conv_Int64ToDouble` (`KismetMathLibrary.RandomInteger64InRange` (`KismetMathLibrary.Conv_DoubleToInt64` _returnvalue_z) -250)))) "AdjustIfPossibleButDontSpawnIfColliding" "OverrideRootScale" null null))
    (:`then_1`
      (`|SpawnActorFromClass` "/Game/JumpGame/BluePrints/stnads_uppers.stnads_uppers_C" (`KismetMathLibrary.MakeTransform` (`KismetMathLibrary.MakeVector` (`KismetMathLibrary.Conv_Int64ToDouble` (`KismetMathLibrary.RandomInteger64InRange` _returnvalue _returnvalue_2)) (`KismetMathLibrary.Conv_Int64ToDouble` (`KismetMathLibrary.RandomInteger64InRange` _returnvalue _returnvalue_2)) (`KismetMathLibrary.Conv_Int64ToDouble` (`KismetMathLibrary.RandomInteger64InRange` -200 200)))) "AdjustIfPossibleButDontSpawnIfColliding" "OverrideRootScale" null _asbp_third_person_character))))

(fn `UserConstructionScript`)